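; BP_SlowZone is a zone actor that shrinks steadily to nothing over the length of a round.
; Construction sets the current radius to the initial radius.
; Each Tick accumulates elapsed time, linearly interpolates the radius toward zero against the maximum round time, clamps it at zero and applies it as uniform actor scale.
; The graphs contain only this shrinking, with no slowing logic.
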(event `self.ReceiveTick`
  (params (DeltaSeconds :type "Float (single-precision)"))
  (bind _currentradius (`self.CurrentRadius`))
  (bind _output_get (set `self.elapsed_time` (+ (`self.elapsed_time`) DeltaSeconds)))
  (set `self.CurrentRadius` (`KismetMathLibrary.Lerp` (`self.InitialRadius`) 0.0 (- 1.0 (/ (- (`self.RoundMaxTime`) _output_get) (`self.RoundMaxTime`)))))
  (if (<= (`self.CurrentRadius`) 0.0)
    (bind _output_get_2 (set `self.CurrentRadius` 0.0))
    (else
      (set `self.CurrentRadius` _currentradius)))
  (`self.SetActorScale3D` (`KismetMathLibrary.Conv_DoubleToVector` _currentradius)))

(fn `UserConstructionScript`
  (set `self.CurrentRadius` (`self.InitialRadius`)))