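; Game mode for a four-player local multiplayer team game, handling player spawning, team tracking and end-of-match checks.
; BeginPlay creates local players, possesses BP_PlayerOne pawns with assigned teams, switches to a shared camera and shows the team-size widget.
; Team events message per-team widgets in a map, print win or tie, and reload the level when kills leave one team.
; The code creating those team widgets is disconnected.
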(event `self.ReceiveBeginPlay`
  (`|ExecutionSequence`
    (:`then_0`
      (`self.SpawnPlayers`)
      (`self.Find Camera Actor`))
    (:`then_1`
      (`PlayerController.SetViewTargetWithBlend` (`GameplayStatics.GetPlayerController` 0) (`self.MainCamera`) 0.0 "VTBlend_Linear" 0.0 false))
    (:`then_2`
      (bind _returnvalue (`|CreateWidget` "/Game/Lukes_Folder/WB_TeamSize.WB_TeamSize_C"))
      (`UserWidget.AddToViewport` _returnvalue 0)
      (set `self.TeamSize_Widget` _returnvalue))))

(event `Find Camera Actor`
  (bind _outactors (`GameplayStatics.GetAllActorsOfClass` "/Game/Yenum/Blueprints/Camera.Camera_C"))
  (set `self.MainCamera` (`|GetArrayItem` _outactors)))

(event `/Game/Lukes_Folder/TeamSize_Interface.PlayerSpawned`
  (params (Team :type Name))
  (bind (_value _returnvalue) (`BlueprintMapLibrary.Map_Find` (`self.Team+Icon_Array`) Team))
  (set `self.CurrentOperatingTeamName` Team)
  (if _returnvalue
    ;[1 1 1] Increa team size in UI
    (message `/Game/Lukes_Folder/TeamSize_Interface.PlayerSpawned` _value Team)))

(event `/Game/Lukes_Folder/TeamSize_Interface.PlayerKilled`
  (params (KilledPlayer :type "Actor Object Reference") (KilledPlayer_TeamName :type Name))
  (bind _team_icon_array (`self.Team+Icon_Array`))
  (bind _currentoperatingteamname (`self.CurrentOperatingTeamName`))
  (`KismetSystemLibrary.PrintString` "Hello")
  (set `self.Amount of Teams` (- (`self.Amount of Teams`) 1))
  (if (<= (`self.Amount of Teams`) 1)
    (bind _returnvalue (`GameplayStatics.GetCurrentLevelName` true))
    (`GameplayStatics.OpenLevel` (`KismetStringLibrary.Conv_StringToName` _returnvalue))
    ;[1 1 1] Find Killed Player Reference
    (set `self.CurrentOperatingTeamName` KilledPlayer_TeamName)
    (bind _keys (`BlueprintMapLibrary.Map_Keys` _team_icon_array))
    (for _array_element _keys
      (if (== _array_element _currentoperatingteamname)
        ;[1 1 1] Tell UI which to remove
        (message `/Game/Lukes_Folder/TeamSize_Interface.PlayerKilled` (`BlueprintMapLibrary.Map_Find` _team_icon_array _array_element) null _currentoperatingteamname)))))

(event `/Game/Lukes_Folder/TeamSize_Interface.TeamLost`
  (params (TeamName :type Name))
  (bind _team_icon_array (`self.Team+Icon_Array`))
  ;[1 1 1] Remove Defeated team from contestested
  (`|ExecutionSequence`
    (:`then_1`
      (`BlueprintMapLibrary.Map_Remove` _team_icon_array TeamName)
      (set `self.Amount of Teams` (`BlueprintMapLibrary.Map_Length` _team_icon_array))
      (bind _keys (`BlueprintMapLibrary.Map_Keys` _team_icon_array))
      (for _array_element _keys
        _)
      (if (== (`self.Amount of Teams`) 1)
        (`KismetSystemLibrary.PrintString` (`KismetStringLibrary.Conv_NameToString` _array_element))
        (`KismetSystemLibrary.PrintString` "Wins")
        (elif (< (`self.Amount of Teams`) 1)
          (`KismetSystemLibrary.PrintString` "Tie"))))))

(fn `SpawnPlayers`
  (for _index (range 1 4)
    (`GameplayStatics.CreatePlayer` _index))
  (for _index_2 (range 4)
    (bind _returnvalue (`|SpawnActorFromClass` "/Game/Yenum/Blueprints/Character/BP_PlayerOne.BP_PlayerOne_C" (`KismetMathLibrary.MakeTransform` (0.0 0.0 2000.0)) "Undefined" "MultiplyWithRoot" null _index_2 (`BlueprintMapLibrary.Map_Find` (`self.AssignedTeam`) _index_2) null))
    (`Controller.Possess` (`GameplayStatics.GetPlayerController` _index_2) _returnvalue)
    (message `/Game/Lukes_Folder/TeamSize_Interface.PlayerSpawned` self (`/Game/Yenum/Blueprints/BP_CharacterBase.TeamName` _returnvalue))))

(fn `UserConstructionScript`)