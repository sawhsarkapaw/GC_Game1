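; BP_PlayerOne is a player character Blueprint that colors itself by player index and registers its spawn with the game mode.
; On BeginPlay it sets one of three mesh materials from PlayerInt, calls SpawnFunction, then after a short delay calls MakeInvisible and sends its TeamName to the game mode.
; An unconnected chain would report the player killed after a random delay and destroy the actor, but it never runs.
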(event `self.ReceiveBeginPlay`
  (`self.SetColor`)
  (`self.SpawnFunction`)
  (`KismetSystemLibrary.Delay` 2.0)
  (`self.Make Invisible`)
  (`|ExecutionSequence`
    (:`then_0`
      (message `/Game/Lukes_Folder/TeamSize_Interface.PlayerSpawned` (`GameplayStatics.GetGameMode`) (`self.TeamName`)))))

(fn `SetColor`
  (switch `int` (`self.PlayerInt`)
    (:`0`
      (`PrimitiveComponent.SetMaterial` (`self.Mesh`) 0 "/Game/Kapaw/Assets/Textures/M_Blue.M_Blue"))
    (:`1`
      (`PrimitiveComponent.SetMaterial` (`self.Mesh`) 0 "/Game/Kapaw/Assets/Textures/M_Red.M_Red"))
    (:`2`
      (`PrimitiveComponent.SetMaterial` (`self.Mesh`) 0 "/Game/LevelPrototyping/Materials/MI_PrototypeGrid_TopDark.MI_PrototypeGrid_TopDark"))))

(fn `UserConstructionScript`
  (`parent.UserConstructionScript`))