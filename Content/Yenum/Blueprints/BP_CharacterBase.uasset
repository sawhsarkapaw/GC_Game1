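; Base player character for a team twin-stick shooter where players turn invisible after spawning and briefly reappear when they fire.
; Enhanced Input drives world-axis movement, stick-direction aiming through control rotation, and shooting with a small bullet count that refills after a short lockout.
; Death reveals and ragdolls the body, disables input and notifies the game mode, which also receives spawn messages.
; SpawnFunction teleports the character to the PlayerStart tagged with its player number.
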(event `self.ReceiveBeginPlay`
  (`KismetSystemLibrary.Delay` (`self.Duration`))
  (message `/Game/Lukes_Folder/TeamSize_Interface.PlayerSpawned` (`GameplayStatics.GetGameMode`) (`self.TeamName`))
  (`KismetSystemLibrary.Delay` 3.0)
  (`self.Make Invisible`))

(event `self.ReceivePossessed`
  (params (NewController :type "Controller Object Reference"))
  (bind _asbp_player_controller_gcs (cast `/Game/Yenum/Game/BP_PlayerController_GCS` NewController))
  (`EnhancedInputSubsystemInterface.AddMappingContext` (pcsubsystem `EnhancedInputLocalPlayerSubsystem` _asbp_player_controller_gcs) "/Game/Yenum/Input/IMC_GCS.IMC_GCS" 0 (struct)))

(event `EnhancedInput|/Game/Yenum/Input/Actions/IA_MOVE_FORWARD_GCS`
  (params (ActionValue :type "Float (double-precision)") (ElapsedSeconds :type "Float (double-precision)") (TriggeredSeconds :type "Float (double-precision)") (InputAction :type "InputAction Object Reference" :default "/Game/Yenum/Input/Actions/IA_MOVE_FORWARD_GCS.IA_MOVE_FORWARD_GCS"))
  ;[1 0.3812 0.9371] Movement
  (:`Triggered`
    (`self.AddMovementInput` (0.0 1.0 0.0) ActionValue)))

(event `EnhancedInput|/Game/Yenum/Input/Actions/IA_MOVE_RIGHT_GCS`
  (params (ActionValue :type "Float (double-precision)") (ElapsedSeconds :type "Float (double-precision)") (TriggeredSeconds :type "Float (double-precision)") (InputAction :type "InputAction Object Reference" :default "/Game/Yenum/Input/Actions/IA_MOVE_RIGHT_GCS.IA_MOVE_RIGHT_GCS"))
  ;[1 0.3812 0.9371] Movement
  (:`Triggered`
    (`self.AddMovementInput` (-1.0 0.0 0.0) ActionValue)))

(event `EnhancedInput|/Game/Yenum/Input/Actions/IA_TURNX_GCS`
  (params (ActionValue :type "Vector2D Structure") (ElapsedSeconds :type "Float (double-precision)") (TriggeredSeconds :type "Float (double-precision)") (InputAction :type "InputAction Object Reference" :default "/Game/Yenum/Input/Actions/IA_TURNX_GCS.IA_TURNX_GCS"))
  (bind _returnvalue (`GameplayStatics.GetPlayerController` (`self.PlayerInt`)))
  (bind _returnvalue_2 (`KismetMathLibrary.MakeRotationFromAxes` (`KismetMathLibrary.MakeVector` ActionValue_X ActionValue_Y)))
  ;[1 0.3812 0.9371] Movement
  (:`Triggered`
    (if (and (<= (`KismetMathLibrary.Abs` (`self.GetInputAxisKeyValue`)) 0.3) (<= (`KismetMathLibrary.Abs` (`self.GetInputAxisKeyValue`)) 0.3))
      (`Controller.SetControlRotation` _returnvalue (`self.RightStickRotation`))
      (else
        (`Controller.SetControlRotation` _returnvalue _returnvalue_2)
        (set `self.RightStickRotation` _returnvalue_2)))))

(event `EnhancedInput|/Game/Yenum/Input/Actions/IA_SHOOT_GCS`
  (params (ActionValue :type Boolean) (ElapsedSeconds :type "Float (double-precision)") (TriggeredSeconds :type "Float (double-precision)") (InputAction :type "InputAction Object Reference" :default "/Game/Yenum/Input/Actions/IA_SHOOT_GCS.IA_SHOOT_GCS"))
  (bind _returnvalue_location (`KismetMathLibrary.BreakTransform` (`self.GetTransform`)))
  (bind _returnvalue (`self.K2_GetActorRotation`))
  ;[1 1 1] Shooting
  (:`Started`
    (if (`self.CanShoot`)
      (`GameplayStatics.PlaySound2D` "/Game/Sound/S_PewPew.S_PewPew" 1.0 1.0 0.0 null null)
      (`KismetSystemLibrary.PrintString` "Shoot")
      (`|SpawnActorFromClass` "/Game/Kapaw/Blueprints/BP_Projectile.BP_Projectile_C" (`KismetMathLibrary.MakeTransform` (+ _returnvalue_location (`KismetMathLibrary.GreaterGreater_VectorRotator` (`self.ProjectileOffset`) _returnvalue)) _returnvalue) "AlwaysSpawn" "MultiplyWithRoot" null null)
      (`self.Make Visible`)
      (bind _result (`/Engine/EditorBlueprintResources/StandardMacros.DecrementInt` (`self.BulletCount`))
        (:`  `
          (set `self.BulletCount` _result)
          (if (<= (`self.BulletCount`) 0)
            (set `self.CanShoot` false)
            (`self.Unlock Shooting`)))))))

(event `Make Invisible`
  (`self.SetActorHiddenInGame` true))

(event `Make Visible`
  (`self.SetActorHiddenInGame` false)
  (if (not (`self.IsDead`))
    (`KismetSystemLibrary.Delay` 1.0)
    (`self.Make Invisible`)))

(event `Unlock Shooting`
  (`KismetSystemLibrary.Delay` 1.0)
  (set `self.CanShoot` true)
  (set `self.BulletCount` 2))

(event `Disable Character Movement`
  (`CharacterMovementComponent.DisableMovement` (`self.CharacterMovement`)))

(event `Enable Character Movement`
  (`KismetSystemLibrary.Delay` 3.0)
  (`CharacterMovementComponent.SetMovementMode` (`self.CharacterMovement`) "MOVE_Walking" 0))

(event `OnDeath`
  (bind _mesh (`self.Mesh`))
  (set `self.IsDead` true)
  (`self.SetActorHiddenInGame` false)
  (`CharacterMovementComponent.DisableMovement` (`self.CharacterMovement`))
  (`self.DisableInput` (`GameplayStatics.GetPlayerController` (`self.PlayerInt`)))
  (`PrimitiveComponent.SetSimulatePhysics` _mesh true)
  (`ActorComponent.K2_DestroyComponent` (`self.CapsuleComponent`))
  (`PrimitiveComponent.SetCollisionResponseToChannel` _mesh "ECC_WorldDynamic" "ECR_Ignore")
  (message `/Game/Lukes_Folder/TeamSize_Interface.PlayerKilled` (`GameplayStatics.GetGameMode`) self (`self.TeamName`)))

(fn `SpawnFunction`
  (bind _outactors (`GameplayStatics.GetAllActorsOfClass` "/Script/Engine.PlayerStart"))
  (for _array_element _outactors
    (if (== (`PlayerStart.PlayerStartTag` _array_element) (`KismetStringLibrary.Concat_StrStr` "P" (`KismetStringLibrary.Conv_IntToString` (`self.PlayerInt`))))
      (bind _output_get (set `self.SpawnLocation` (`self.GetTransform` _array_element)))
      (`self.K2_SetActorTransform` _output_get false true))))

(fn `UserConstructionScript`)