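; BP_InvisibleZone is a moving trigger zone that notifies actors as they enter and leave its box.
; Box overlap begin and end send InZone1Visible and OutZone1Visible messages to the other actor.
; On BeginPlay, a timeline at play rate Rate moves the zone to PositionToMoveTo, lerping from its current location each update, so motion compounds rather than following the curve directly.
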(event `self.ReceiveBeginPlay`
  (`self.StartMovingIn`))

(event `self.Box.OnComponentBeginOverlap`
  (params (OverlappedComponent :type "PrimitiveComponent Object Reference") (OtherActor :type "Actor Object Reference") (OtherComp :type "PrimitiveComponent Object Reference") (OtherBodyIndex :type Integer) (bFromSweep :type Boolean) (SweepResult :type "HitResult Structure (by ref)"))
  (message `/Game/Kapaw/Interfaces/BPI_Character.In_Zone1_Visible` OtherActor))

(event `self.Box.OnComponentEndOverlap`
  (params (OverlappedComponent :type "PrimitiveComponent Object Reference") (OtherActor :type "Actor Object Reference") (OtherComp :type "PrimitiveComponent Object Reference") (OtherBodyIndex :type Integer))
  (message `/Game/Kapaw/Interfaces/BPI_Character.Out_Zone1_Visible` OtherActor))

(event `StartMovingIn`
  (`TimelineComponent.SetPlayRate` (`self.Timeline`) (`self.Rate`))
  (bind (_direction _float_track) (`Timeline|Timeline` :!via `PlayFromStart`)
    (:`Update`
      (`self.K2_SetActorLocation` (`KismetMathLibrary.VLerp` (`self.K2_GetActorLocation`) (`self.PositionToMoveTo`) _float_track)))))

(fn `UserConstructionScript`)